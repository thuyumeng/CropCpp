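; GS_Railling is a Geometry Script generated-mesh Blueprint that builds a round railing bar along a spline.
; On mesh rebuild, it creates a circle profile from Radius and Roundess, and offsets Spline by Height into HelperSpline.
; It samples HelperSpline uniformly in time, with the count derived from Subdivitions and point count.
; The circle is swept along those frames into the target mesh.
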(event Events|EventOnRebuildGeneratedMesh
  (params (TargetMesh :type Dynamic%20Mesh%20Object%20Reference))
  (bind _helper_spline (Variables|Default|GetHelper%20Spline))
  (Utilities|FlowControl|Sequence
    (:then_0
      (bind _returnvalue (Class|GeometryScriptLibraryPolyPathFunctions|CreateCirclePath2D "(X=0.000000,Y=0.000000)" (Variables|Default|GetRadius) (Variables|Default|GetRoundess)))
      (Variables|Default|SetBrush _returnvalue))
    (:then_1
      (Class|GeometryHelper|CreateOffsetedSpline (Variables|Default|GetHelper%20Spline) (Variables|Default|GetSpline) (Math|Vector|MakeVector 0.0 0.0 (Variables|Default|Getheight))))
    (:then_2
      (bind _frames (Class|GeometryScriptLibraryPolyPathFunctions|SampleSplinetoTransforms :Spline _helper_spline :SamplingOptions (Utilities|Struct|MakeGeometryScriptSplineSamplingOptions (Math|Float|Truncate (|(((1+Subs)*(Points-1))+1) (Math|Conversions|ToFloat(Integer) (Variables|Default|GetSubdivitions)) (Math|Conversions|ToFloat(Integer) (Spline|GetNumberOfSplinePoints _helper_spline)))) 1.0 "UniformTime" "Local")))
      (Class|GeometryScriptLibraryMeshPrimitiveFunctions|AppendSweepPolygon :TargetMesh TargetMesh :PolygonVertices (Class|GeometryScriptLibraryPolyPathFunctions|ToArrayOfVector2D(GeometryScriptPolyPath) (Variables|Default|GetBrush)) :SweepPath _frames :Debug 0))))

(fn ConstructionScript)